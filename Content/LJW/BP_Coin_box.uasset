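; BP_Coin_box is a coin pickup that the VR player collects by touching its sphere trigger.
; On overlap with BP_VR_Player it plays a coin sound and increments the Coin count stored in MD_GameInstance.
; It then writes the new total to the player's coin number text component and destroys itself.
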(event `self.Sphere.OnComponentBeginOverlap`
  (params (OverlappedComponent :type "PrimitiveComponent Object Reference") (OtherActor :type "Actor Object Reference") (OtherComp :type "PrimitiveComponent Object Reference") (OtherBodyIndex :type Integer) (bFromSweep :type Boolean) (SweepResult :type "HitResult Structure (by ref)"))
  (bind _asbp_vr_player (cast `/Game/KDH/Blueprints/BP_VR_Player` OtherActor))
  (`GameplayStatics.PlaySound2D` "/Game/LJW/sound/effect/Coins_Single_00.Coins_Single_00" 1.0 1.0 0.0 null null)
  (bind _asmd_game_instance (cast `MD_GameInstance` (`GameplayStatics.GetGameInstance`)))
  (bind _result (`/Engine/EditorBlueprintResources/StandardMacros.IncrementInt` (`MD_GameInstance.coin` _asmd_game_instance))
    (:`  `
      (bind _output_get (set `MD_GameInstance.coin` _result _asmd_game_instance))
      (`TextRenderComponent.K2_SetText` (`VR_Player.textCompCoinNum` _asbp_vr_player) (`KismetTextLibrary.Conv_IntToText` _output_get))
      (`self.K2_DestroyActor`))))

(fn `UserConstructionScript`)