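; BP_NPC_2 is an NPC that shows a widget when the VR player comes near.
; The widget starts hidden; entering the Box trigger reveals it and sets the TEXT flag on its WG_NPC_2 instance.
; Leaving the box hides the widget and pulses the End flag on the ABP_NPC_2 anim instance for one second.
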(event `self.ReceiveBeginPlay`
  (`SceneComponent.SetVisibility` (`self.Widget`) false false))

(event `self.Box.OnComponentBeginOverlap`
  (params (OverlappedComponent :type "PrimitiveComponent Object Reference") (OtherActor :type "Actor Object Reference") (OtherComp :type "PrimitiveComponent Object Reference") (OtherBodyIndex :type Integer) (bFromSweep :type Boolean) (SweepResult :type "HitResult Structure (by ref)"))
  (cast `/Game/KDH/Blueprints/BP_VR_Player` OtherActor)
  (`SceneComponent.SetVisibility` (`self.Widget`) true false)
  (bind _aswg_npc_2 (cast `/Game/LJW/UI/WG_NPC_2` (`WidgetComponent.GetWidget` (`self.Widget`))))
  (set `/Game/LJW/UI/WG_NPC_2.TEXT` true _aswg_npc_2))

(event `self.Box.OnComponentEndOverlap`
  (params (OverlappedComponent :type "PrimitiveComponent Object Reference") (OtherActor :type "Actor Object Reference") (OtherComp :type "PrimitiveComponent Object Reference") (OtherBodyIndex :type Integer))
  (cast `/Game/KDH/Blueprints/BP_VR_Player` OtherActor)
  (`SceneComponent.SetVisibility` (`self.Widget`) false false)
  (bind _asabp_npc_2 (cast `/Game/LJW/NPC/Anim/elf/ABP_NPC_2` (`SkeletalMeshComponent.GetAnimInstance` (`self.Mesh`))))
  (set `/Game/LJW/NPC/Anim/elf/ABP_NPC_2.End` true _asabp_npc_2)
  (`KismetSystemLibrary.Delay` 1.0)
  (set `/Game/LJW/NPC/Anim/elf/ABP_NPC_2.End` false _asabp_npc_2))

(fn `UserConstructionScript`)