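; Level music controller actor that switches background tracks as the VR player moves between zones and triggers a boss encounter.
; It plays an opening track on BeginPlay, swaps to another while the player overlaps Box, and restarts the first on exit.
; Entering BoxBOss, gated by a boolean that is then cleared, spawns BP_Enemy_king after a short delay and replaces the post-exit track with boss music.
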(event `self.ReceiveBeginPlay`
  (bind _returnvalue (`GameplayStatics.SpawnSound2D` "/Game/LJW/sound/back/01__Curious.01__Curious" 1.0 1.0 0.0 null)))

(event `self.Box.OnComponentBeginOverlap`
  (params (OverlappedComponent :type "PrimitiveComponent Object Reference") (OtherActor :type "Actor Object Reference") (OtherComp :type "PrimitiveComponent Object Reference") (OtherBodyIndex :type Integer) (bFromSweep :type Boolean) (SweepResult :type "HitResult Structure (by ref)"))
  (cast `/Game/KDH/Blueprints/BP_VR_Player` OtherActor)
  (`AudioComponent.Stop` (stale `self.ReceiveBeginPlay` _returnvalue))
  (bind _returnvalue (`GameplayStatics.SpawnSound2D` "/Game/LJW/sound/back/TRACK_2.TRACK_2" 1.0 1.0 0.0 null)))

(event `self.Box.OnComponentEndOverlap`
  (params (OverlappedComponent :type "PrimitiveComponent Object Reference") (OtherActor :type "Actor Object Reference") (OtherComp :type "PrimitiveComponent Object Reference") (OtherBodyIndex :type Integer))
  (cast `/Game/KDH/Blueprints/BP_VR_Player` OtherActor)
  (`AudioComponent.Stop` (stale `self.Box.OnComponentBeginOverlap` _returnvalue))
  (bind _returnvalue (`GameplayStatics.SpawnSound2D` "/Game/LJW/sound/back/01__Curious.01__Curious" 1.0 1.0 0.0 null)))

(event `self.BoxBOss.OnComponentBeginOverlap`
  (params (OverlappedComponent :type "PrimitiveComponent Object Reference") (OtherActor :type "Actor Object Reference") (OtherComp :type "PrimitiveComponent Object Reference") (OtherBodyIndex :type Integer) (bFromSweep :type Boolean) (SweepResult :type "HitResult Structure (by ref)"))
  (cast `/Game/KDH/Blueprints/BP_VR_Player` OtherActor)
  (if (`self.NewVar_0`)
    (`KismetSystemLibrary.Delay` 1.0)
    (`|SpawnActorFromClass` "/Game/LJW/BP_Enemy_king.BP_Enemy_king_C" (`KismetMathLibrary.MakeTransform` (`self.NewVar`) (struct :`Yaw` 90.0)) "AlwaysSpawn" "OverrideRootScale" null null)
    (set `self.NewVar_0` false)
    (`AudioComponent.Stop` (stale `self.Box.OnComponentEndOverlap` _returnvalue))
    (`GameplayStatics.SpawnSound2D` "/Game/LJW/sound/back/TRACK_4.TRACK_4" 1.0 1.0 0.0 null)))

(fn `UserConstructionScript`)