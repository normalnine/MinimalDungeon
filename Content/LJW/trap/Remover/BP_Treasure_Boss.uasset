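; BP_Treasure_Boss is a treasure chest that the VR player opens by spending a key from the game instance.
; Overlapping its box with a key decrements the count, updates the player's key text and swings the lid open on a timeline.
; After a delay, a first-time flag allows one coin box plus a random bomb, pear or red potion.
; Later overlaps still consume keys; construction applies the treasure material.
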(event `self.ReceiveActorEndOverlap`
  (params (OtherActor :type "Actor Object Reference"))
  ;[1 1 1] close
)

(event `ClosedChest`
  ;[1 1 1] close
)

(event `self.ReceiveActorBeginOverlap`
  (params (OtherActor :type "Actor Object Reference"))
  ;[1 1 1] open
  ;;[1 1 1] old
)

(event `OpenChest`
  ;[1 1 1] open
  (bind (_direction _lidopen) (`Timeline|Lid_Open`)
    (:`Update`
      (`SceneComponent.K2_SetRelativeRotation` (`self.Lid`) (* (struct :`Roll` -120.0) _lidopen) false false))))

(event `self.Box.OnComponentBeginOverlap`
  (params (OverlappedComponent :type "PrimitiveComponent Object Reference") (OtherActor :type "Actor Object Reference") (OtherComp :type "PrimitiveComponent Object Reference") (OtherBodyIndex :type Integer) (bFromSweep :type Boolean) (SweepResult :type "HitResult Structure (by ref)"))
  (bind _returnvalue (+ (`self.K2_GetActorLocation`) (0.0 100.0 100.0)))
  (bind _returnvalue_2 (`KismetMathLibrary.Conv_VectorToTransform` _returnvalue))
  ;[1 1 1] open
  (bind _asbp_vr_player (cast `/Game/KDH/Blueprints/BP_VR_Player` OtherActor))
  (bind _asmd_game_instance (cast `MD_GameInstance` (`GameplayStatics.GetGameInstance`)))
  (if (> (`MD_GameInstance.key` _asmd_game_instance) 0)
    (bind _output_get (set `MD_GameInstance.key` (- (`MD_GameInstance.key` _asmd_game_instance) 1) _asmd_game_instance))
    (`TextRenderComponent.K2_SetText` (`VR_Player.textCompKeyNum` _asbp_vr_player) (`KismetTextLibrary.Conv_IntToText` _output_get))
    (`self.OpenChest`)
    (if (`self.one`)
      (`KismetSystemLibrary.Delay` 1.0)
      (set `self.one` false)
      (`|SpawnActorFromClass` "/Game/LJW/BP_Coin_box.BP_Coin_box_C" (`KismetMathLibrary.Conv_VectorToTransform` (+ (`self.K2_GetActorLocation`) (10.0 100.0 100.0))) "AlwaysSpawn" "OverrideRootScale" null null)
      (switch `int` (`KismetMathLibrary.RandomIntegerInRange` 0 2)
        (:`0`
          (`|SpawnActorFromClass` "/Game/KDH/Blueprints/BP_Bomb.BP_Bomb_C" _returnvalue_2 "AlwaysSpawn" "OverrideRootScale" null null))
        (:`1`
          (`|SpawnActorFromClass` "/Game/KDH/Blueprints/BP_Pear.BP_Pear_C" (`KismetMathLibrary.MakeTransform` _returnvalue (struct :`Yaw` -90.0)) "AlwaysSpawn" "OverrideRootScale" null null))
        (:`2`
          (`|SpawnActorFromClass` "/Game/KDH/Blueprints/BP_Potion_Red.BP_Potion_Red_C" _returnvalue_2 "AlwaysSpawn" "OverrideRootScale" null null))))))

(fn `UserConstructionScript`
  (bind _treasure_material (`self.Treasure Material`))
  (`PrimitiveComponent.SetMaterial` (`self.Base`) 0 _treasure_material)
  (`PrimitiveComponent.SetMaterial` (`self.Lid`) 0 _treasure_material)
  (`PrimitiveComponent.SetMaterial` (`self.Treasure`) 0 _treasure_material))