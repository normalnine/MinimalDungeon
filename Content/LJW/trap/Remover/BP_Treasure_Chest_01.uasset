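; Treasure chest that opens when the VR player enters its trigger box and yields a coin box.
; The overlap calls OpenChest, whose Lid_Open timeline rotates the lid, then after a short delay spawns BP_Coin_box above the chest, guarded by a one-time flag.
; The construction script applies TreasureMaterial to the base, lid and treasure.
; Closing is unimplemented, and the older actor-overlap logic is disconnected.
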(event `self.ReceiveActorEndOverlap`
  (params (OtherActor :type "Actor Object Reference"))
  ;[1 1 1] close
)

(event `ClosedChest`
  ;[1 1 1] close
)

(event `self.ReceiveActorBeginOverlap`
  (params (OtherActor :type "Actor Object Reference"))
  ;[1 1 1] open
  ;;[1 1 1] old
)

(event `OpenChest`
  ;[1 1 1] open
  (bind (_direction _lidopen) (`Timeline|Lid_Open`)
    (:`Update`
      (`SceneComponent.K2_SetRelativeRotation` (`self.Lid`) (* (struct :`Roll` -120.0) _lidopen) false false))))

(event `self.Box.OnComponentBeginOverlap`
  (params (OverlappedComponent :type "PrimitiveComponent Object Reference") (OtherActor :type "Actor Object Reference") (OtherComp :type "PrimitiveComponent Object Reference") (OtherBodyIndex :type Integer) (bFromSweep :type Boolean) (SweepResult :type "HitResult Structure (by ref)"))
  ;[1 1 1] open
  (cast `/Game/KDH/Blueprints/BP_VR_Player` OtherActor)
  (`self.OpenChest`)
  (if (`self.one`)
    (`KismetSystemLibrary.Delay` 0.5)
    (`|SpawnActorFromClass` "/Game/LJW/BP_Coin_box.BP_Coin_box_C" (`KismetMathLibrary.Conv_VectorToTransform` (+ (`self.K2_GetActorLocation`) (30.0 0.0 100.0))) "AlwaysSpawn" "OverrideRootScale" null null)
    (set `self.one` false)))

(fn `UserConstructionScript`
  (bind _treasure_material (`self.Treasure Material`))
  (`PrimitiveComponent.SetMaterial` (`self.Base`) 0 _treasure_material)
  (`PrimitiveComponent.SetMaterial` (`self.Lid`) 0 _treasure_material)
  (`PrimitiveComponent.SetMaterial` (`self.Treasure`) 0 _treasure_material))