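; Saw blade trap that travels along a spline and damages the VR player on contact.
; The MoveSawBlade timeline starts on BeginPlay, mapping its Distance track to spline length to place the blade.
; Blade pitch and yaw follow the spline, while the timeline's Rotation track drives roll for spin.
; Capsule overlap with BP_VR_Player calls ReceiveDamage and applies a very small launch.
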(event `self.ReceiveBeginPlay`
  (bind _sawblade (`self.SawBlade`))
  (bind _sawbladepatch (`self.SawBladePatch`))
  (bind (_direction _distance _rotation) (`Timeline|MoveSawBlade`)
    (:`Update`
      (bind _returnvalue (* _distance (`SplineComponent.GetSplineLength` _sawbladepatch)))
      (`SceneComponent.K2_SetWorldLocation` _sawblade (`SplineComponent.GetLocationAtDistanceAlongSpline` _sawbladepatch _returnvalue "World") false false)
      (bind (_returnvalue_roll _returnvalue_pitch _returnvalue_yaw) (`KismetMathLibrary.BreakRotator` (`SplineComponent.GetRotationAtDistanceAlongSpline` _sawbladepatch _returnvalue "Local")))
      (`SceneComponent.K2_SetRelativeRotation` _sawblade (`KismetMathLibrary.MakeRotator` _rotation _returnvalue_pitch _returnvalue_yaw) false false))))

(event `self.ReceiveActorBeginOverlap`
  (params (OtherActor :type "Actor Object Reference")))

(event `self.Capsule.OnComponentBeginOverlap`
  (params (OverlappedComponent :type "PrimitiveComponent Object Reference") (OtherActor :type "Actor Object Reference") (OtherComp :type "PrimitiveComponent Object Reference") (OtherBodyIndex :type Integer) (bFromSweep :type Boolean) (SweepResult :type "HitResult Structure (by ref)"))
  (bind _asbp_vr_player (cast `/Game/KDH/Blueprints/BP_VR_Player` OtherActor))
  (`VR_Player.ReceiveDamage` _asbp_vr_player)
  (`Character.LaunchCharacter` _asbp_vr_player (0.5 0.5 0.5) false false))

(fn `UserConstructionScript`)